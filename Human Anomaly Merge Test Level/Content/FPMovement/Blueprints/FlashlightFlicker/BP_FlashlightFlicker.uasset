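; Placeable trigger that makes the first-person player's flashlight flicker on overlap, with box dimensions set in the construction script.
; BeginPlay caches the player; the first overlap plays a timeline scaling spotlight intensity between zero and its normal value, if the flashlight is on.
; DoOnce precedes the player and flashlight checks, so any first overlap consumes the trigger.
; An animated montage variant is unfinished and never runs.
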(event OnComponentBeginOverlap(TriggerBox)
  (params (OverlappedComponent :type Primitive%20Component%20Object%20Reference) (OtherActor :type Actor%20Object%20Reference) (OtherComp :type Primitive%20Component%20Object%20Reference) (OtherBodyIndex :type Integer) (bFromSweep :type Boolean) (SweepResult :type Hit%20Result%20Structure%20%28by%20ref%29))
  ;[0.05098 0.05098 0.05098] Flashlight Flicker function
  (Utilities|FlowControl|DoOnce false
    (:Completed
      (bind _asbp_fpmovement_player (Utilities|Casting|CastToBP_FPMovementPlayer OtherActor))
      (if (Variables|/Game/FPMovement/Player/Blueprints/BP_FPMovementPlayer.BP_FPMovementPlayer_C|GetFlashlightOn? _asbp_fpmovement_player)
        (if true
          ;;[0.05098 0.05098 0.05098] without Animation
          (bind _alpha (Timeline|Flicker_TL Play)
            (:Update
              (Rendering|Components|Light|SetIntensity (Variables|/Game/FPMovement/Player/Blueprints/BP_FPMovementPlayer.BP_FPMovementPlayer_C|GetSpotLight (Variables|Reference|GetPlayer%20Reference)) (Math|Float|Lerp 0.0 (Variables|/Game/FPMovement/Player/Blueprints/BP_FPMovementPlayer.BP_FPMovementPlayer_C|GetFlashlightIntensity (Variables|Reference|GetPlayer%20Reference)) _alpha)))))))))

(event EventBeginPlay
  ;[0.05098 0.05098 0.05098] Cast to Player
  (bind _asbp_fpmovement_player (Utilities|Casting|CastToBP_FPMovementPlayer (Game|GetPlayerCharacter 0)))
  (Variables|Reference|SetPlayer%20Reference _asbp_fpmovement_player))

(fn ConstructionScript
  (Transformation|SetWorldScale3D (Variables|Default|GetTriggerBox) (Math|Vector|MakeVector (Variables|FlickerSettings|GetBox%20Length) (Variables|FlickerSettings|GetBox%20Thickness) (Variables|FlickerSettings|GetBox%20Height))))